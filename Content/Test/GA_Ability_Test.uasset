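; Test gameplay ability that damages one nearby combat-capable actor, with on-screen prints and debug drawing.
; On activation, a zero-length sphere trace on Visibility runs at the avatar's location, ignoring the avatar.
; A hit implementing CombatInterface receives a damage effect built from class defaults, and the ability then ends on input release.
; Any other result ends the ability after a short delay.
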(event `self.K2_ActivateAbility`
  (bind _returnvalue (`self.GetAvatarActorFromActorInfo`))
  (bind _returnvalue_2 (`Actor.K2_GetActorLocation` _returnvalue))
  (`KismetSystemLibrary.PrintString` (`KismetSystemLibrary.GetDisplayName` _returnvalue))
  (bind (_outhit _returnvalue_3) (`KismetSystemLibrary.SphereTraceSingle` _returnvalue_2 _returnvalue_2 100.0 "TraceTypeQuery1" false (`|MakeArray` _returnvalue) "ForDuration" true (struct :`R` 1.0 :`A` 1.0) (struct :`G` 1.0 :`A` 1.0) 1.0))
  (if _returnvalue_3
    (bind (_bblockinghit _binitialoverlap _time _distance _location _impactpoint _normal _impactnormal _physmat _hitactor) (`GameplayStatics.BreakHitResult` _outhit))
    (if (`KismetSystemLibrary.DoesImplementInterface` _hitactor "/Script/ProjectG.CombatInterface")
      (`AbilitySystemLibrary.ApplyDamageEffect` (`self.MakeDamageEffectParamsFromClassDefaults` _hitactor))
      (`AbilityTask_WaitInputRelease.WaitInputRelease` false
        (:`OnRelease`
          (`self.K2_EndAbility`)))
      (else
        (`KismetSystemLibrary.Delay` 0.2 :!label _label)
        (`self.K2_EndAbility`)))
    (else
      (goto _label))))

(event `self.K2_OnEndAbility`
  (params (bWasCancelled :type Boolean))
  (`KismetSystemLibrary.PrintString` "End Ability"))